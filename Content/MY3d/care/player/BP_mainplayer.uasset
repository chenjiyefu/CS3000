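; BP_mainplayer is the player character, with jumping, camera-relative planar movement, mouse-look and pickup tracking.
; On BeginPlay it shows the cursor and opens the Begin widget.
; AddCoin updates the coin count on a text render component, while GetAKey stores keys as gameplay tags and prints the container.
; Entercelebration switches the Playerstart enum state and attaches a Niagara celebration effect to the capsule.
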(event EventBeginPlay
  (Variables|/Script/Engine.PlayerController|SetbShowMouseCursor (Game|GetPlayerController 0) true)
  (bind _returnvalue (UserInterface|CreateWidget "/Game/MY3d/care/UI/begin.begin_C"))
  (UserInterface|Viewport|AddtoViewport _returnvalue 0))

(event Input|ActionEvents|InputActionjump
  (params (Key :type Key%20Structure :default "None"))
  ;[1 1 1] 跳跃
  (:Pressed
    (Character|Jump))
  (:Released
    (Character|StopJumping)))

(event Input|AxisEvents|InputAxis前后
  (params (AxisValue :type Float%20%28single-precision%29))
  (bind _returnvalue (Pawn|GetControlRotation :!class /Script/Engine.Pawn))
  (bind _returnvalue_2 (Math|Vector|GetForwardVector _returnvalue))
  ;[1 1 1] 移动
  (Pawn|Input|AddMovementInput (Math|Vector|MakeVector (.x _returnvalue_2) (.y _returnvalue_2) 0.0) AxisValue false))

(event Input|AxisEvents|InputAxis左右
  (params (AxisValue :type Float%20%28single-precision%29))
  (bind _returnvalue (Pawn|GetControlRotation :!class /Script/Engine.Pawn))
  (bind _returnvalue_2 (Math|Vector|GetRightVector _returnvalue))
  ;[1 1 1] 移动
  (Pawn|Input|AddMovementInput (Math|Vector|MakeVector (.x _returnvalue_2) (.y _returnvalue_2) 0.0) AxisValue false))

(event Input|AxisEvents|InputAxisturn
  (params (AxisValue :type Float%20%28single-precision%29))
  ;[1 1 1] 相机移动
  (Pawn|Input|AddControllerYawInput AxisValue))

(event Input|AxisEvents|InputAxislookup
  (params (AxisValue :type Float%20%28single-precision%29))
  ;[1 1 1] 相机移动
  (Pawn|Input|AddControllerPitchInput AxisValue))

(fn ConstructionScript)

(fn AddCoin
  (bind _output_get (Variables|Default|SetCOIN (+ (Variables|Default|GetCOIN) 1)))
  (Rendering|Components|TextRender|SetText (Variables|Default|GetTextRender) (Utilities|Text|ToText(Integer) _output_get)))

(fn GetAKey
  (params (keytodbtain :type Gameplay%20Tag%20Structure))
  (bind _key (Variables|Default|Getkey))
  (GameplayTags|AddGameplayTag _key keytodbtain :!class /Script/GameplayTags.BlueprintGameplayTagLibrary)
  (Development|PrintString (GameplayTags|GetDebugStringfromGameplayTagContainer _key)))

(fn Entercelebration
  (Variables|Default|Setplayerstart "NewEnumerator2")
  (Niagara|SpawnSystemAttached "/Game/TeachersMarketplace/Assets/VFX/Emitters/Character/NS_Celebrate.NS_Celebrate" (Variables|Collision|GetCapsuleComponent) "None" "0, 0, 0" "0, 0, 0" "SnapToTarget" false))