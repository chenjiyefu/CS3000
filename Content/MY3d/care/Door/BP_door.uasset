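; BP_door is a force-field door that opens for a player holding a matching key.
; On BeginPlay it creates a dynamic force-field material on the mesh and applies its configured color.
; When BP_mainplayer overlaps the box, its Key tag container is tested against the door's Getkey tag query.
; A match immediately disables mesh collision and plays a timeline that drives the material's Opacity; no logic closes it again.
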(event OnComponentBeginOverlap(Box)
  (params (OverlappedComponent :type Primitive%20Component%20Object%20Reference) (OtherActor :type Actor%20Object%20Reference) (OtherComp :type Primitive%20Component%20Object%20Reference) (OtherBodyIndex :type Integer) (bFromSweep :type Boolean) (SweepResult :type Hit%20Result%20Structure%20%28by%20ref%29))
  (bind _asbp_mainplayer (Utilities|Casting|CastToBP_mainplayer OtherActor))
  (if (GameplayTags|DoesContainerMatchTagQuery (Variables|/Game/MY3d/care/player/BP_mainplayer.BP_mainplayer_C|Getkey _asbp_mainplayer) (Variables|Default|Getgetkey))
    (CallFunction|打开大门)))

(event Custom|打开大门
  (Collision|SetCollisionEnabled (Variables|Default|GetStaticMesh1) "NoCollision")
  (bind _新建轨道_0 (Timeline|时间轴 Play)
    (:Update
      (Rendering|Material|SetScalarParameterValue (Variables|Default|Get动态材质) "Opacity" _新建轨道_0 :!class /Script/Engine.MaterialInstanceDynamic))))

(event EventBeginPlay
  (bind _returnvalue (Rendering|Material|CreateDynamicMaterialInstance (Variables|Default|GetStaticMesh1) 0 "/Game/TeachersMarketplace/Assets/Architecture/Gate/Material/MI_forcefield.MI_forcefield" "None" :!class /Script/Engine.PrimitiveComponent))
  (Variables|Default|Set动态材质 _returnvalue)
  (Rendering|Material|SetVectorParameterValue (Variables|Default|Get动态材质) "ColorMultiplier" (Variables|Default|Get动态材质颜色) :!class /Script/Engine.MaterialInstanceDynamic))

(event Collision|EventActorBeginOverlap
  (params (OtherActor :type Actor%20Object%20Reference)))

(event EventTick
  (params (DeltaSeconds :type Float%20%28single-precision%29)))

(fn ConstructionScript)