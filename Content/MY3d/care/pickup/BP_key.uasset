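; BP_key is a key pickup that grants a key to the player who collects it.
; It overrides the parent's PickedThisUp event, calls the parent logic, then casts the collector to BP_mainplayer and passes its Keytype to GetAKey.
; BeginPlay, overlap and Tick are disabled stubs, and the construction script only calls its parent.
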(event EventBeginPlay
  (|CallParentFunction) ; 此节点被禁用，将不会被调用。\n从引脚连出引线来编译功能。
)

(event Collision|EventActorBeginOverlap
  (params (OtherActor :type Actor%20Object%20Reference))
  (|CallParentFunction OtherActor) ; 此节点被禁用，将不会被调用。\n从引脚连出引线来编译功能。
)

(event EventTick
  (params (DeltaSeconds :type Float%20%28single-precision%29))
  (|CallParentFunction DeltaSeconds) ; 此节点被禁用，将不会被调用。\n从引脚连出引线来编译功能。
)

(event EventPickedThisUp
  (params (actorthatpickedthisup :type Actor%20Object%20Reference))
  (|CallParentFunction actorthatpickedthisup)
  (bind _asbp_mainplayer (Utilities|Casting|CastToBP_mainplayer actorthatpickedthisup))
  (Default|GetAKey _asbp_mainplayer (Variables|Default|Getkeytype)))

(fn ConstructionScript
  (|CallParentFunction))