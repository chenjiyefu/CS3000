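; BP_hightspawn_4 is an NPC pawn that chases the player and sends actors touching its Box back to the respawn point.
; From BeginPlay it loops AI MoveTo toward the player, retrying on failure and playing the APS_NPC attack montage on arrival before moving again.
; Box overlap teleports any overlapping actor, unfiltered, to the 重生点 (respawn point) location and rotation stored in MYgamemode, independently of the attack.
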(event OnComponentBeginOverlap(Box)
  (params (OverlappedComponent :type Primitive%20Component%20Object%20Reference) (OtherActor :type Actor%20Object%20Reference) (OtherComp :type Primitive%20Component%20Object%20Reference) (OtherBodyIndex :type Integer) (bFromSweep :type Boolean) (SweepResult :type Hit%20Result%20Structure%20%28by%20ref%29))
  (bind _asmygamemode (Utilities|Casting|CastToMYgamemode (Game|GetGameMode)))
  (Transformation|Teleport OtherActor (.location (Variables|/Game/MY3d/care/BP/MYgamemode.MYgamemode_C|Get重生点 _asmygamemode)) (.rotation (Variables|/Game/MY3d/care/BP/MYgamemode.MYgamemode_C|Get重生点 _asmygamemode))))

(event Custom|attack
  (Animation|Montage|PlayMontage (Variables|Default|GetSkeletalMesh) "/Game/MY3d/care/Animation/NPC/Animation_NPC/APS_NPC.APS_NPC"
    (:OnCompleted
      (CallFunction|Move))))

(event Custom|MOVE
  (AI|AIMoveTo self "0, 0, 0" (Game|GetPlayerCharacter 0) 7e+01 false
    (:OnSuccess
      (CallFunction|Attack))
    (:OnFail
      (CallFunction|Move))))

(event EventBeginPlay
  (CallFunction|MOVE))

(event Collision|EventActorBeginOverlap
  (params (OtherActor :type Actor%20Object%20Reference)))

(event EventTick
  (params (DeltaSeconds :type Float%20%28single-precision%29)))

(fn ConstructionScript)